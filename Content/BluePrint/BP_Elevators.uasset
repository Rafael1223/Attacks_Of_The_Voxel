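; BP_Elevators is a one-way elevator actor that the player triggers through an interact event.
; Its box overlap shows a WBP_Interact prompt until exit, and creates it only while the elevator has not been used.
; InteractElevator fires once, driving timelines that press and re-material the button, move two referenced door actors and move the elevator between start and end points.
; Each timeline starts from the previous one's Update, so the motions overlap.
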(event OnComponentBeginOverlap(Box)
  (params (OverlappedComponent :type Primitive%20Component%20Object%20Reference) (OtherActor :type Actor%20Object%20Reference) (OtherComp :type Primitive%20Component%20Object%20Reference) (OtherBodyIndex :type Integer) (bFromSweep :type Boolean) (SweepResult :type Hit%20Result%20Structure%20%28by%20ref%29))
  ;[1 1 1] Interact Prompt
  (if (not (Variables|Default|GetIsElevatorUp))
    (if (not (Variables|Default|GetElevator_HUD?))
      (bind _returnvalue (UserInterface|CreateWidget "/Game/BluePrint/Widget/WBP_Interact.WBP_Interact_C"))
      (Variables|/Game/BluePrint/Widget/WBP_Interact.WBP_Interact_C|SetInteract%20Text _returnvalue (Variables|Default|GetInteract%20Text))
      (UserInterface|Viewport|AddtoViewport _returnvalue 0)
      (Variables|Default|SetElevator_HUD? true))))

(event OnComponentEndOverlap(Box)
  (params (OverlappedComponent :type Primitive%20Component%20Object%20Reference) (OtherActor :type Actor%20Object%20Reference) (OtherComp :type Primitive%20Component%20Object%20Reference) (OtherBodyIndex :type Integer))
  ;[1 1 1] Interact Prompt
  (Widget|RemovefromParent (stale OnComponentBeginOverlap(Box) _returnvalue))
  (Variables|Default|SetElevator_HUD? false))

(event EventBeginPlay)

(event Collision|EventActorBeginOverlap
  (params (OtherActor :type Actor%20Object%20Reference)))

(event EventTick
  (params (DeltaSeconds :type Float%20%28single-precision%29)))

(event EventInteractElevator
  (bind _button (Variables|Default|GetButton))
  ;[1 1 1] Comment
  (Utilities|FlowControl|DoOnce false
    (:Completed
      (Variables|Default|SetIsElevatorUp true)
      (bind _button_2 (Timeline|Buttan_Timeline Play)
        (:Update
          (Transformation|SetRelativeLocation _button (Math|Vector|Lerp(Vector) (Variables|Button|GetButton%20Normal) (Variables|Button|GetButton%20Down) _button_2) false false)
          (Rendering|Material|SetMaterial _button 0 "/Game/Important_Assets/Polar/Materials/Cloth/_M_Master_Rubber._M_Master_Rubber")
          (bind _doors_l (Timeline|DoorLeft%20_Timeline Play)
            (:Update
              (Transformation|SetActorLocation (Variables|DoorObj|GetDoor%20L) (Math|Vector|Lerp(Vector) (Variables|MovingDoors|GetDoorL_Start%20Point) (Variables|MovingDoors|GetDoorL_End%20Point) _doors_l) false false)
              (bind _doors_r (Timeline|DoorRight_TimeLine Play)
                (:Update
                  (Transformation|SetActorLocation (Variables|DoorObj|GetDoor%20R) (Math|Vector|Lerp(Vector) (Variables|MovingDoors|GetDoorR_Start%20Point) (Variables|MovingDoors|GetDoorR_End%20Point) _doors_r) false false)
                  (bind _elevator_up (Timeline|ElevatorUP_Timeline Play)
                    (:Update
                      (Transformation|SetActorRelativeLocation (Math|Vector|Lerp(Vector) (Variables|ElevatorPoints|GetElevator%20Start%20Point) (Variables|ElevatorPoints|GetElevator%20End%20%20Point) _elevator_up)))))))))))))

(fn ConstructionScript)