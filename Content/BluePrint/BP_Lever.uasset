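; Interactable lever that swings a referenced Door actor open, with an on-screen interact prompt for the player.
; A Box trigger shows WBP_Interact when BP_FirstPersonCharacter enters, guarded by the LeverHUD flag, and removes it when any overlap ends.
; InteractLever plays a sound and a timeline that rotates the Head component.
; That timeline's Update drives a second timeline that rotates the door between preset rotations.
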(event OnComponentBeginOverlap(Box)
  (params (OverlappedComponent :type Primitive%20Component%20Object%20Reference) (OtherActor :type Actor%20Object%20Reference) (OtherComp :type Primitive%20Component%20Object%20Reference) (OtherBodyIndex :type Integer) (bFromSweep :type Boolean) (SweepResult :type Hit%20Result%20Structure%20%28by%20ref%29))
  ;[1 1 1] Interact Prompt
  (if (== (Utilities|GetClass OtherActor) "/Game/Important_Assets/FirstPerson/Blueprints/BP_FirstPersonCharacter.BP_FirstPersonCharacter_C")
    (if (not (Variables|Default|GetLever_HUD?))
      (bind _returnvalue (UserInterface|CreateWidget "/Game/BluePrint/Widget/WBP_Interact.WBP_Interact_C"))
      (Variables|/Game/BluePrint/Widget/WBP_Interact.WBP_Interact_C|SetInteract%20Text _returnvalue (Variables|Default|GetInteract%20Text))
      (UserInterface|Viewport|AddtoViewport _returnvalue 0)
      (Variables|Default|SetLever_HUD? true))))

(event OnComponentEndOverlap(Box)
  (params (OverlappedComponent :type Primitive%20Component%20Object%20Reference) (OtherActor :type Actor%20Object%20Reference) (OtherComp :type Primitive%20Component%20Object%20Reference) (OtherBodyIndex :type Integer))
  ;[1 1 1] Interact Prompt
  (Widget|RemovefromParent (stale OnComponentBeginOverlap(Box) _returnvalue))
  (Variables|Default|SetLever_HUD? false))

(event EventInteractLever
  ;[1 1 1] Move Lever/Door
  (Audio|PlaySoundatLocation "/Game/Audio/SFX/S_inspect-item.S_inspect-item" (Transformation|GetActorLocation) "0, 0, 0" 1.0 1.0 0.0 0 0 0 0)
  (bind _newtrack_0 (Timeline|MoveLever_Timeline Play)
    (:Update
      (Transformation|SetRelativeRotation (Variables|Default|GetHead) (Math|Rotator|Lerp(Rotator) (Variables|MoveLever|GetLever%20Rotation%20Beginning) (Variables|MoveLever|GetLever%20Rotation%20End) _newtrack_0) false false)
      (bind _newtrack_0_2 (Timeline|OpenDoor_Timeline Play)
        (:Update
          (Transformation|SetActorRotation (Variables|Default|GetDoor) (Math|Rotator|Lerp(Rotator) (Variables|MoveDoor|GetMove%20Exit%20Door%20Beginning) (Variables|MoveDoor|GetMove%20Exit%20Door%20End) _newtrack_0_2)))))))

(fn ConstructionScript)