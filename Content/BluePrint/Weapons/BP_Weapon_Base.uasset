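; Base weapon Blueprint providing hitscan firing and reloading for the first-person player.
; Fire line-traces from player 0's camera with debug drawing, spends ammo without checking the count, and subtracts damage directly from any BP_MechSoldier hit.
; Hits spawn an explosion, enlarged on a kill when the soldier is destroyed.
; Reload tops up the clip from reserve ammo and flags the character as reloading, or prints a full-ammo message.
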(event Custom|Fire
  ;[1 1 1] Fire the Gun
  (bind _asbp_first_person_character (Utilities|Casting|CastToBP_FirstPersonCharacter (Game|GetPlayerCharacter 0)))
  (bind _outhit (Collision|LineTraceByChannel (Transformation|GetWorldLocation (Variables|/Game/Important_Assets/FirstPerson/Blueprints/BP_FirstPersonCharacter.BP_FirstPersonCharacter_C|GetFirstPersonCamera _asbp_first_person_character)) (+ (Transformation|GetWorldLocation (Variables|/Game/Important_Assets/FirstPerson/Blueprints/BP_FirstPersonCharacter.BP_FirstPersonCharacter_C|GetFirstPersonCamera _asbp_first_person_character)) (* (Math|Vector|GetForwardVector (Transformation|GetWorldRotation (Variables|/Game/Important_Assets/FirstPerson/Blueprints/BP_FirstPersonCharacter.BP_FirstPersonCharacter_C|GetFirstPersonCamera _asbp_first_person_character))) (Variables|Default|GetRange))) "TraceTypeQuery1" false 0 "ForDuration"))
  (Variables|Default|SetAmmo (- (Variables|Default|GetAmmo) 1))
  (bind _asbp_mech_soldier (Utilities|Casting|CastToBP_MechSoldier (.HitActor (Collision|BreakHitResult _outhit))))
  (Variables|/Game/BluePrint/Enemy/BP_MechSoldier.BP_MechSoldier_C|SetIsHit? _asbp_mech_soldier true)
  (bind _output_get (Variables|/Game/BluePrint/Enemy/BP_MechSoldier.BP_MechSoldier_C|SetHeath _asbp_mech_soldier (- (Variables|/Game/BluePrint/Enemy/BP_MechSoldier.BP_MechSoldier_C|GetHeath _asbp_mech_soldier) (Variables|Default|GetDamage))))
  (if (<= _output_get 0.0)
    (Effects|SpawnEmitteratLocation "/Game/Important_Assets/StarterContent/Particles/P_Explosion.P_Explosion" (.Location (Collision|BreakHitResult _outhit)) "0, 0, 0" "4.000000,4.000000,4.000000")
    (Actor|DestroyActor _asbp_mech_soldier)
    (else
      (Effects|SpawnEmitteratLocation "/Game/Important_Assets/StarterContent/Particles/P_Explosion.P_Explosion" (.Location (Collision|BreakHitResult _outhit))))))

(event EventBeginPlay)

(event Collision|EventActorBeginOverlap
  (params (OtherActor :type Actor%20Object%20Reference)))

(event EventTick
  (params (DeltaSeconds :type Float%20%28single-precision%29)))

(fn ConstructionScript)

(fn Reload
  (if (< (Variables|Default|GetAmmo) (Variables|Default|GetClipSize))
    (if (> (Variables|Default|GetMaxAmmo) (- (Variables|Default|GetClipSize) (Variables|Default|GetAmmo)))
      (Variables|Default|SetAmmoDifference (- (Variables|Default|GetClipSize) (Variables|Default|GetAmmo)))
      (Variables|Default|SetAmmo (+ (Variables|Default|GetAmmo) (Variables|Default|GetAmmoDifference)))
      (Variables|Default|SetMaxAmmo (- (Variables|Default|GetMaxAmmo) (Variables|Default|GetAmmoDifference)))
      (bind _asbp_first_person_character (Utilities|Casting|CastToBP_FirstPersonCharacter (Game|GetPlayerCharacter 0)))
      (Variables|/Game/Important_Assets/FirstPerson/Blueprints/BP_FirstPersonCharacter.BP_FirstPersonCharacter_C|SetIsReloading? _asbp_first_person_character true)
      (else
        (Variables|Default|SetAmmoDifference (- (Variables|Default|GetClipSize) (Variables|Default|GetAmmo)))
        (Variables|Default|SetAmmo (+ (Variables|Default|GetAmmo) (Variables|Default|GetMaxAmmo)))
        (Variables|Default|SetMaxAmmo 0)
        (bind _asbp_first_person_character_2 (Utilities|Casting|CastToBP_FirstPersonCharacter (Game|GetPlayerCharacter 0)))
        (Variables|/Game/Important_Assets/FirstPerson/Blueprints/BP_FirstPersonCharacter.BP_FirstPersonCharacter_C|SetIsReloading? _asbp_first_person_character_2 true)))
    (else
      (Development|PrintString "Full Ammo"))))