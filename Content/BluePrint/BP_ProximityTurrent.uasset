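; Proximity turret that raises its neck and turns its head toward the player while they are inside a detection sphere; no firing logic is present.
; Sphere overlaps trigger Activate or Deactive, which move the neck through FindPlayer, a lerp loop using frame-length delays.
; Once raised, Combat_Timeline updates drive the smoothed look-at rotation, stopping after the neck lowers.
; Construction gives the eye a tinted dynamic material, and BeginPlay sizes and shows the sphere.
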(event OnComponentBeginOverlap(Sphere)
  (params (OverlappedComponent :type Primitive%20Component%20Object%20Reference) (OtherActor :type Actor%20Object%20Reference) (OtherComp :type Primitive%20Component%20Object%20Reference) (OtherBodyIndex :type Integer) (bFromSweep :type Boolean) (SweepResult :type Hit%20Result%20Structure%20%28by%20ref%29))
  ;[1 1 1] Activate and deactivate the Turrets when the player enters the sphere
  (if (== OtherActor (Game|GetPlayerCharacter 0))
    (CallFunction|Activate)))

(event OnComponentEndOverlap(Sphere)
  (params (OverlappedComponent :type Primitive%20Component%20Object%20Reference) (OtherActor :type Actor%20Object%20Reference) (OtherComp :type Primitive%20Component%20Object%20Reference) (OtherBodyIndex :type Integer))
  ;[1 1 1] Activate and deactivate the Turrets when the player enters the sphere
  (if (== OtherActor (Game|GetPlayerCharacter 0))
    (CallFunction|Deactive)))

(event Custom|Activate
  (Utilities|FindPlayer "0,0,100.000000"
    (:End
      (Timeline|Combat_Timeline Play
        (:Update
          (CallFunction|LookatPlayer))))))

(event Custom|Deactive
  (Utilities|FindPlayer "0,0,0.000000"
    (:End
      (Timeline|Combat_Timeline Stop
        (:Update
          (CallFunction|LookatPlayer))))))

(event EventBeginPlay
  (bind _sphere (Variables|Default|GetSphere))
  ;[0 0.7079 1] Event BeginPlay
  (Components|Sphere|SetSphereRadius _sphere (Variables|Default|GetSphere%20Radius) true)
  (Development|SetHiddeninGame _sphere false false))

(fn ConstructionScript
  (bind _returnvalue (Rendering|Material|CreateDynamicMaterialInstance (Variables|Default|GetEye) 0 "/Game/Materials/M_HeathPack.M_HeathPack" "None" :!class /Script/Engine.PrimitiveComponent))
  (bind _output_get (Variables|Default|SetEye%20Material%20REF _returnvalue))
  (Rendering|Material|SetVectorParameterValue _output_get "Color" (Variables|Default|GetEye%20Clolor) :!class /Script/Engine.MaterialInstanceDynamic))

(fn LookatPlayer
  (bind _head (Variables|Default|GetHead))
  (Transformation|SetWorldRotation _head (Math|Rotator|Lerp(Rotator) (Transformation|GetWorldRotation _head) (Math|Rotator|FindLookatRotation (Transformation|GetWorldLocation (Variables|Default|GetHead)) (Transformation|GetActorLocation (Game|Player|GetPlayerPawn 0))) 0.5) false false))