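; BP_MechSoldier is a melee enemy that roams, chases the first-person player and deals damage.
; A looping timer sends it to random reachable points within its patrol radius, or toward the player if it was hit.
; Pawn sensing turns the eye material and light to the alert color and starts a chase-and-attack loop.
; Reaching the player opens a timed attack window in which collision overlap damages once.
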(event OnSeePawn(PawnSensing)
  (params (Pawn :type Pawn%20Object%20Reference))
  ;[1 1 1] See Player
  (CallFunction|UpdateEyeColor (Variables|Eye|GetEye%20Color%20Activate))
  (bind _asbp_first_person_character (Utilities|Casting|CastToBP_FirstPersonCharacter Pawn))
  (Variables|Default|SetCanSeePlayer? false)
  (AI|AIMoveTo self "0, 0, 0" _asbp_first_person_character 5.0 false :!label _label
    (:OnSuccess
      (if (not (Variables|Default|GetIsAttacking?))
        (Variables|Default|SetIsAttacking? true)
        (Utilities|FlowControl|Delay 2.67)
        (Variables|Default|SetIsAttacking? false)
        (Variables|Default|SetAlraedyHit? false)
        (goto _label)))))

(event OnComponentBeginOverlap(AttackingCollision)
  (params (OverlappedComponent :type Primitive%20Component%20Object%20Reference) (OtherActor :type Actor%20Object%20Reference) (OtherComp :type Primitive%20Component%20Object%20Reference) (OtherBodyIndex :type Integer) (bFromSweep :type Boolean) (SweepResult :type Hit%20Result%20Structure%20%28by%20ref%29))
  ;[1 1 1] Attacking Player
  (bind _asbp_first_person_character (Utilities|Casting|CastToBP_FirstPersonCharacter OtherActor))
  (if (Variables|Default|GetIsAttacking?)
    (if (not (Variables|Default|GetAlraedyHit?))
      (Default|DamagePlayer _asbp_first_person_character 0.2)
      (Variables|Default|SetAlraedyHit? true))))

(event Custom|Roaming
  ;[1 1 1] Roaming Event
  (|Roaming_CollapseGraph))

(event EventBeginPlay
  ;[0 0.9642 1] BegianPlay
  (Components|Sphere|SetSphereRadius (Variables|Default|GetRadius%20Sphere) (Variables|Default|GetPatrol%20%20Radius) true)
  ;[1 1 1] Roaming Event
  (Utilities|Time|SetTimerbyEvent (delegate Custom|Roaming) 3.0 true))

(fn ConstructionScript
  ;[1 1 1] Eye Material
  (bind _returnvalue (Rendering|Material|CreateDynamicMaterialInstance (Variables|Default|GetEye) 0 "/Game/Materials/M_LightIndicator.M_LightIndicator" "None" :!class /Script/Engine.PrimitiveComponent))
  (bind _output_get (Variables|Eye|SetEye%20Material%20REF _returnvalue))
  (Rendering|Material|SetVectorParameterValue _output_get "Color" (Variables|Eye|GetEye%20Color%20Deactive) :!class /Script/Engine.MaterialInstanceDynamic)
  ;[1 1 1] Eye Color
  (Rendering|Components|Light|SetLightColor (Variables|Default|GetPointLight) (Variables|Eye|GetEye%20Color%20Deactive) true))

(fn UpdateEyeColor
  (params (Color :type Linear%20Color%20Structure))
  (Rendering|Material|SetVectorParameterValue (Variables|Eye|GetEye%20Material%20REF) "Color" Color :!class /Script/Engine.MaterialInstanceDynamic)
  (Rendering|Components|Light|SetLightColor (Variables|Default|GetPointLight) Color true))