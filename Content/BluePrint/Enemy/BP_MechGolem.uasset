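; Enemy mech golem that patrols, chases the player and self-destructs in an explosion on reaching them.
; A looping timer triggers Roaming, which moves to random reachable points within PatrolRadius, or toward the player when MechGolemIsHit is set.
; Pawn sensing switches eye color and retries AIMoveTo until success, then destroys the golem, spawns the explosion and subtracts ExplosionDamage directly from player health.
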(event OnSeePawn(PawnSensing)
  (params (Pawn :type Pawn%20Object%20Reference))
  ;[1 1 1] See Player
  (CallFunction|UpdateEyeColor (Variables|Eye|GetEye%20Color%20Activate))
  (bind _asbp_first_person_character (Utilities|Casting|CastToBP_FirstPersonCharacter Pawn))
  (Variables|Default|SetCanSeePlayer? false)
  (AI|AIMoveTo self "0, 0, 0" _asbp_first_person_character 5.0 false :!label _label
    (:OnSuccess
      (Variables|Default|SetMechGolem_AlraedyHit? false)
      (Actor|DestroyActor)
      (Effects|SpawnEmitteratLocation "/Game/Important_Assets/StarterContent/Particles/P_Explosion.P_Explosion" (Transformation|GetActorLocation) "0, 0, 0" "2.000000,2.000000,2.000000")
      (Variables|/Game/Important_Assets/FirstPerson/Blueprints/BP_FirstPersonCharacter.BP_FirstPersonCharacter_C|SetHeath _asbp_first_person_character (- (Variables|/Game/Important_Assets/FirstPerson/Blueprints/BP_FirstPersonCharacter.BP_FirstPersonCharacter_C|GetHeath _asbp_first_person_character) (Variables|Default|GetExplosion%20Damage))))
    (:OnFail
      (goto _label))))

(event Custom|Roaming
  ;[0 0.4068 1] BeginPlay
  (|Roaming_CollapseGraph_2))

(event EventBeginPlay
  ;[0 0.4068 1] BeginPlay
  (Components|Sphere|SetSphereRadius (Variables|Default|GetRadius%20Sphere) (Variables|Default|GetPatrol%20%20Radius) true)
  (Utilities|Time|SetTimerbyEvent (delegate Custom|Roaming) 3.0 true))

(fn ConstructionScript)

(fn UpdateEyeColor
  (params (Color :type Linear%20Color%20Structure))
  (Rendering|Material|SetVectorParameterValue (Variables|Eye|GetEye%20Material%20REF) "Color" Color :!class /Script/Engine.MaterialInstanceDynamic)
  (Rendering|Components|Light|SetLightColor (Variables|Default|GetPointLight) Color true))