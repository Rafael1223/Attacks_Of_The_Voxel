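; BP_KeyCard is a key card pickup that grants the first-person character a key.
; Overlapping its Box with that character shows a WBP_Interact prompt, removed on end overlap.
; InteractKeyCard inserts true into the character's HasKey array at index KeycardValue, then destroys the card.
; The construction script tints dynamic instances of M_HeathPack and M_Key, both created on mesh element 0, so the second replaces the first.
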(event OnComponentBeginOverlap(Box)
  (params (OverlappedComponent :type Primitive%20Component%20Object%20Reference) (OtherActor :type Actor%20Object%20Reference) (OtherComp :type Primitive%20Component%20Object%20Reference) (OtherBodyIndex :type Integer) (bFromSweep :type Boolean) (SweepResult :type Hit%20Result%20Structure%20%28by%20ref%29))
  ;[1 1 1] Interact Prompt
  (if (== (Utilities|GetClass OtherActor) "/Game/Important_Assets/FirstPerson/Blueprints/BP_FirstPersonCharacter.BP_FirstPersonCharacter_C")
    (if (not (Variables|Default|GetKeyCard_HUD?))
      (bind _returnvalue (UserInterface|CreateWidget "/Game/BluePrint/Widget/WBP_Interact.WBP_Interact_C"))
      (Variables|/Game/BluePrint/Widget/WBP_Interact.WBP_Interact_C|SetInteract%20Text _returnvalue (Variables|Default|GetInteract%20Text))
      (UserInterface|Viewport|AddtoViewport _returnvalue 0)
      (Variables|Default|SetKeyCard_HUD? true))))

(event OnComponentEndOverlap(Box)
  (params (OverlappedComponent :type Primitive%20Component%20Object%20Reference) (OtherActor :type Actor%20Object%20Reference) (OtherComp :type Primitive%20Component%20Object%20Reference) (OtherBodyIndex :type Integer))
  ;[1 1 1] Interact Prompt
  (Widget|RemovefromParent (stale OnComponentBeginOverlap(Box) _returnvalue))
  (Variables|Default|SetKeyCard_HUD? false))

(event EventInteractKeyCard
  ;[1 1 1] Interact Key
  (bind _asbp_first_person_character (Utilities|Casting|CastToBP_FirstPersonCharacter (stale OnComponentEndOverlap(Box) OtherActor)))
  (Utilities|Array|Insert (Variables|/Game/Important_Assets/FirstPerson/Blueprints/BP_FirstPersonCharacter.BP_FirstPersonCharacter_C|GetHasKey? _asbp_first_person_character) true (Variables|Default|GetKeycard%20Value))
  (Components|DestroyComponent (Variables|Default|GetKeyCard))
  (Actor|DestroyActor))

(fn ConstructionScript
  (bind _returnvalue (Rendering|Material|CreateDynamicMaterialInstance (Variables|Default|GetKeyCard) 0 "/Game/Materials/M_HeathPack.M_HeathPack" "" :!class /Script/Engine.PrimitiveComponent))
  (bind _output_get (Variables|REF|SetKeyCard%20light%20REF _returnvalue))
  (Rendering|Material|SetVectorParameterValue _output_get "Color" (Variables|Colors|GetKeyCard%20light%20Color) :!class /Script/Engine.MaterialInstanceDynamic)
  (bind _returnvalue_2 (Rendering|Material|CreateDynamicMaterialInstance (Variables|Default|GetKeyCard) 0 "/Game/Materials/M_Key.M_Key" "" :!class /Script/Engine.PrimitiveComponent))
  (bind _output_get_2 (Variables|REF|SetKeyCard%20Mat%20REF _returnvalue_2))
  (Rendering|Material|SetVectorParameterValue _output_get_2 "Key Color" (Variables|Colors|GetKeyCard%20Color) :!class /Script/Engine.MaterialInstanceDynamic))