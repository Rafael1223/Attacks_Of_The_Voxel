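; Base weapon Blueprint that fires projectiles and manages clip and reserve ammo.
; Fire spawns a first-person projectile at the skeletal mesh's Muzzle socket and decrements Ammo, with no empty-clip check inside the event.
; Reload tops up the clip from the MaxAmmo reserve, using whatever remains when the reserve is short, or prints a message when the clip is already full.
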(event Custom|Fire
  ;[1 1 1] Fire the Gun
  (Game|SpawnActorfromClass "/Game/Important_Assets/FirstPerson/Blueprints/BP_FirstPersonProjectile.BP_FirstPersonProjectile_C" (Transformation|GetSocketTransform (Variables|Default|GetSkeletalMesh) "Muzzle" "RTS_World") "Undefined" 0 0)
  (Variables|Default|SetAmmo (- (Variables|Default|GetAmmo) 1)))

(event EventBeginPlay)

(event Collision|EventActorBeginOverlap
  (params (OtherActor :type Actor%20Object%20Reference)))

(event EventTick
  (params (DeltaSeconds :type Float%20%28single-precision%29)))

(fn ConstructionScript)

(fn Reload
  (if (< (Variables|Default|GetAmmo) (Variables|Default|GetClipSize))
    (if (> (Variables|Default|GetMaxAmmo) (- (Variables|Default|GetClipSize) (Variables|Default|GetAmmo)))
      (Variables|Default|SetAmmoDifference (- (Variables|Default|GetClipSize) (Variables|Default|GetAmmo)))
      (Variables|Default|SetAmmo (+ (Variables|Default|GetAmmo) (Variables|Default|GetAmmoDifference)))
      (Variables|Default|SetMaxAmmo (- (Variables|Default|GetMaxAmmo) (Variables|Default|GetAmmoDifference)))
      (else
        (Variables|Default|SetAmmoDifference (- (Variables|Default|GetClipSize) (Variables|Default|GetAmmo)))
        (Variables|Default|SetAmmo (+ (Variables|Default|GetAmmo) (Variables|Default|GetMaxAmmo)))
        (Variables|Default|SetMaxAmmo 0)))
    (else
      (Development|PrintString "Full Ammo"))))