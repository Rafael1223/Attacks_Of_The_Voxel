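; Key-card locked door that opens when the first-person character interacts while holding the key matching its KeyCardValue.
; A box overlap shows an interact prompt, and InteractDoor checks the character's HasKey array, briefly displaying the required key's name on a mismatch.
; Opening plays a sound and a timeline that rotates the pivot, then clears that key slot.
; The construction script tints the door's key indicator through a dynamic material.
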(event OnComponentBeginOverlap(Box)
  (params (OverlappedComponent :type Primitive%20Component%20Object%20Reference) (OtherActor :type Actor%20Object%20Reference) (OtherComp :type Primitive%20Component%20Object%20Reference) (OtherBodyIndex :type Integer) (bFromSweep :type Boolean) (SweepResult :type Hit%20Result%20Structure%20%28by%20ref%29))
  ;[1 1 1] Interact Prompt
  (if (not (Variables|Default|GetIsDoorOpen?))
    (if (not (Variables|Default|GetDoor_HUD?))
      (bind _returnvalue (UserInterface|CreateWidget "/Game/BluePrint/Widget/WBP_Interact.WBP_Interact_C"))
      (Variables|/Game/BluePrint/Widget/WBP_Interact.WBP_Interact_C|SetInteract%20Text _returnvalue (Variables|Default|GetInteract%20Text))
      (UserInterface|Viewport|AddtoViewport _returnvalue 0)
      (Variables|Default|SetDoor_HUD? true))))

(event OnComponentEndOverlap(Box)
  (params (OverlappedComponent :type Primitive%20Component%20Object%20Reference) (OtherActor :type Actor%20Object%20Reference) (OtherComp :type Primitive%20Component%20Object%20Reference) (OtherBodyIndex :type Integer))
  ;[1 1 1] Interact Prompt
  (Widget|RemovefromParent (stale OnComponentBeginOverlap(Box) _returnvalue))
  (Variables|Default|SetDoor_HUD? false))

(event Custom|Open%20Door
  ;[1 1 1] Play the opening animation for the door
  (Variables|Default|SetIsDoorOpen? true)
  (Audio|PlaySoundatLocation "/Game/Audio/SFX/SC_Door_Locked.SC_Door_Locked" (Transformation|GetActorLocation) "0, 0, 0" 1.0 1.0 0.8 0 0 0 0)
  (bind _opendoor_track (Timeline|Door%20Open PlayFromStart)
    (:Update
      (Transformation|SetRelativeRotation (Variables|Default|GetPivot) (Math|Rotator|Lerp(Rotator) (Variables|Default|GetClosed) (Variables|Default|GetOpen) _opendoor_track) false false))
    (:Finished
      (Utilities|FlowControl|Delay 0.2)
      (Utilities|Array|SetArrayElem (Variables|/Game/Important_Assets/FirstPerson/Blueprints/BP_FirstPersonCharacter.BP_FirstPersonCharacter_C|GetHasKey? (stale EventInteractDoor _asbp_first_person_character)) (Variables|Key|GetKeyCard%20Value) false))))

(event EventInteractDoor
  ;[1 1 1] Check to see if you have the key card for this specific door and open it
  (bind _asbp_first_person_character (Utilities|Casting|CastToBP_FirstPersonCharacter (stale OnComponentBeginOverlap(Box) OtherActor)))
  (Utilities|FlowControl|DoOnce false :!label _label
    (:Completed
      (bind (_array_element _array_index) (Utilities|Array|ForEachLoopwithBreak (Variables|/Game/Important_Assets/FirstPerson/Blueprints/BP_FirstPersonCharacter.BP_FirstPersonCharacter_C|GetHasKey? _asbp_first_person_character) :!label _label_2)
        (:LoopBody
          (if (and _array_element (== _array_index (Variables|Key|GetKeyCard%20Value)))
            (CallFunction|OpenDoor)
            (Variables|/Game/BluePrint/Widget/WBP_Key_Name.WBP_Key_Name_C|SetKey%20Name (Variables|Key|GetKey%20Name%20Ref) "")
            (goto _label_2 Break)
            (else
              (|NeedsKey_CollapseGraph))))
        (:Completed
          (if (not (and _array_element (== _array_index (Variables|Key|GetKeyCard%20Value))))
            (Utilities|FlowControl|Sequence
              (:then_0
                (Utilities|FlowControl|DoOnce false))
              (:then_1
                (goto _label Reset)))))))))

(fn ConstructionScript
  ;[1 1 1] Eye Material
  (bind _returnvalue (Rendering|Material|CreateDynamicMaterialInstance (Variables|Default|GetDoor%20Key) 0 "/Game/Materials/M_LightIndicator.M_LightIndicator" "None" :!class /Script/Engine.PrimitiveComponent))
  (bind _output_get (Variables|Key|SetDoor%20Key%20Mat%20Ref _returnvalue))
  (Rendering|Material|SetVectorParameterValue _output_get "Color" (Variables|Key|GetDoor%20Key%20Color) :!class /Script/Engine.MaterialInstanceDynamic))