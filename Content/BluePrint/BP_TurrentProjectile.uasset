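; BP_TurrentProjectile is a turret projectile that damages the first-person player and explodes on impact.
; On BeginPlay it caches the player character through GetActorOfClass.
; When its Projectile component hits an actor of exactly that character class, it calls DamagePlayer on the cached reference.
; Every hit spawns an explosion emitter and sound at the component's location, then destroys the actor.
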(event OnComponentHit(Projectile)
  (params (HitComponent :type Primitive%20Component%20Object%20Reference) (OtherActor :type Actor%20Object%20Reference) (OtherComp :type Primitive%20Component%20Object%20Reference) (NormalImpulse :type Vector :default "0, 0, 0") (Hit :type Hit%20Result%20Structure%20%28by%20ref%29))
  (bind _projectile (Variables|Default|GetProjectile))
  (bind _returnvalue (Transformation|GetWorldLocation _projectile))
  (if (== (Utilities|GetClass OtherActor) "/Game/Important_Assets/FirstPerson/Blueprints/BP_FirstPersonCharacter.BP_FirstPersonCharacter_C")
    (Default|DamagePlayer (Variables|Default|GetPlayer%20REF) (Variables|Default|GetDamage)))
  (Effects|SpawnEmitteratLocation "/Game/Important_Assets/StarterContent/Particles/P_Explosion.P_Explosion" _returnvalue)
  (Audio|SpawnSoundatLocation "/Game/Important_Assets/StarterContent/Audio/Explosion01.Explosion01" _returnvalue "0, 0, 0" 1.0 1.0 0.0 0 0)
  (Actor|DestroyActor))

(event EventBeginPlay
  ;[0 1 1] BeginPlay
  (bind _returnvalue (Actor|GetActorOfClass "/Game/Important_Assets/FirstPerson/Blueprints/BP_FirstPersonCharacter.BP_FirstPersonCharacter_C"))
  (Variables|Default|SetPlayer%20REF _returnvalue))

(fn ConstructionScript)